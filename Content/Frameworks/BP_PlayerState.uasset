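; BP_PlayerState is a player state that tracks a player's name, kills, deaths and dead flag.
; On BeginPlay, for a local player controller, it loads the PlayerSaveInfo save slot and passes the saved name to SentMyNameToServer, which stores it.
; AddKill and AddDeath events increment the counters, with AddDeath also marking the player dead.
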(event Custom|AddKill
  (Math|Integer|IncrementInt (Variables|Default|GetKills)))

(event Custom|AddDeath
  (Math|Integer|IncrementInt (Variables|Default|GetDeaths)
    (:%20%20
      (Variables|Default|SetisDead true))))

(event Custom|Sent%20My%20Name%20To%20Server
  (params (MyName :type Text))
  (Variables|Default|SetMyName MyName))

(event EventBeginPlay
  (if (Pawn|IsLocalPlayerController (Game|GetPlayerController))
    (bind _returnvalue (SaveGame|LoadGamefromSlot "info"))
    (bind _asplayer_save_info (Utilities|Casting|CastToPlayerSaveInfo _returnvalue))
    (CallFunction|SentMyNametoServer (Variables|/Game/Start/PlayerSaveInfo.PlayerSaveInfo_C|GetPlayer%20Name _asplayer_save_info))))

(event EventTick
  (params (DeltaSeconds :type Float%20%28single-precision%29)))

(fn ConstructionScript)